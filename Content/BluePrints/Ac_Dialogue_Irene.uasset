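; Dialogue for the NPC Irène Gu, who advises the player on learning English at ESTIAM through 7speaking or congratulates a TOEIC score.
; Overrides Dialogue, calls the parent, then switches on DialogueTreeIndex into hardcoded AddDialogue nodes branching on the chosen option.
; Branch endings set the tree index or remove or clear dialogue progress, then close the conversation.
; Once the 7speaking advice is accepted, the next tree plays one of two random one-liners.
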(fn Dialogue
  (|CallParentFunction)
  (switch int (Variables|Default|GetDialogueTreeIndex)
    (:0
      (bind (_state _optionindex) (CallFunction|AddDialogue "Irène Gu" "Bonjour, vous semblez stressé, évitez de trop bouger vos bras.. Comment puis-je vous aider ? " (Utilities|Array|MakeArray "Bonjour, j'aimerais m'améliorer en anglais, comment faire ?" "Bonjour, j'ai eu mon TOEIC avec 930 de score !!")))
      (switch Utilities|FlowControl|Switch|SwitchonEnum_DialogState _state
        (:NewEnumerator0
          (switch int _optionindex
            (:0
              (bind (_state_2 _optionindex_2) (CallFunction|AddDialogue "Irène Gu" "Good initiative sir ! Do you know 7speaking ?" (Utilities|Array|MakeArray "Yes i know, is it free ?" "???? In french please !")))
              (switch Utilities|FlowControl|Switch|SwitchonEnum_DialogState _state_2
                (:NewEnumerator0
                  (switch int _optionindex_2
                    (:0
                      (bind _state_3 (CallFunction|AddDialogue "Irène Gu" "Yes it is for all ESTIAM students, you have already an account, use it to improve your english ! " (Utilities|Array|MakeArray "Nice, thank you !")))
                      (switch Utilities|FlowControl|Switch|SwitchonEnum_DialogState _state_3
                        (:NewEnumerator0
                          (CallFunction|SetDialogTreeIndex 1)
                          (CallFunction|CloseConversation))))
                    (:1
                      (bind _state_4 (CallFunction|AddDialogue "Irène Gu" "NO FRENCH SIR !! Oh my god, you can't even understand those few sentences.. what a shame.." (Utilities|Array|MakeArray "-.-")))
                      (switch Utilities|FlowControl|Switch|SwitchonEnum_DialogState _state_4
                        (:NewEnumerator0
                          (CallFunction|RemoveDialogueProgress 2)
                          (CallFunction|CloseConversation))))))))
            (:1
              (bind _state_5 (CallFunction|AddDialogue "Irène Gu" "OH MY GOD !! CONGRATULATIONS SIR ! YOU DESERVE IT ! " (Utilities|Array|MakeArray "ahah thank you !")))
              (switch Utilities|FlowControl|Switch|SwitchonEnum_DialogState _state_5
                (:NewEnumerator0
                  (CallFunction|ClearDialogueProgress)
                  (CallFunction|CloseConversation))))))))
    (:1
      (bind _state_6 (CallFunction|AddDialogue "Irène Gu" (Utilities|Select :Index (Math|Random|RandomIntegerinRange 0 1) :Option%200 "MAKE ESTIAM GREAT AGAIN" :Option%201 "Oh you still here, go learn boy !") (Utilities|Array|MakeArray "Ok..")))
      (switch Utilities|FlowControl|Switch|SwitchonEnum_DialogState _state_6
        (:NewEnumerator0
          (CallFunction|ClearDialogueProgress)
          (CallFunction|CloseConversation))))))