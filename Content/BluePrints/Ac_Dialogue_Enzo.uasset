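; Dialogue component for the NPC Enzo Danthon, a French-language conversation about justifying an absence and asking about the campus-cup.
; The Dialogue override calls its parent, then switches on DialogueTreeIndex and chains AddDialogue nodes that branch on the chosen option.
; Showing a sick note sets the tree to index 1, where Enzo gives one of two random dismissive lines.
; Other endings clear or roll back dialogue progress before closing the conversation.
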(fn Dialogue
  (|CallParentFunction)
  (switch int (Variables|Default|GetDialogueTreeIndex)
    (:0
      (bind (_state _optionindex) (CallFunction|AddDialogue "Enzo Danthon" "Salut ça va ?" (Utilities|Array|MakeArray "Nickel et toi ? Je viens justifier mon absence de la semaine dernière." "ça va et toi ? Le prochain campus-cup est prévu pour quand ?")))
      (switch Utilities|FlowControl|Switch|SwitchonEnum_DialogState _state
        (:NewEnumerator0
          (switch int _optionindex
            (:0
              (bind (_state_2 _optionindex_2) (CallFunction|AddDialogue "Enzo Danthon" "ça marche, t'as un justificatif pour ton absence ? " (Utilities|Array|MakeArray "J'ai un mon arrêt maladie, tiens." "J'étais malade mais je ne suis pas allé voir le médecin parce que j'avais déjà des médicaments chez moi.")))
              (switch Utilities|FlowControl|Switch|SwitchonEnum_DialogState _state_2
                (:NewEnumerator0
                  (switch int _optionindex_2
                    (:0
                      (bind _state_3 (CallFunction|AddDialogue "Enzo Danthon" "*lis l'arrêt*.. C'est good, considère que c'est justifié !" (Utilities|Array|MakeArray "Merci !")))
                      (switch Utilities|FlowControl|Switch|SwitchonEnum_DialogState _state_3
                        (:NewEnumerator0
                          (CallFunction|SetDialogTreeIndex 1)
                          (CallFunction|CloseConversation))))
                    (:1
                      (bind _state_4 (CallFunction|AddDialogue "Enzo Danthon" "Donc tu n'as pas de justificatif.. Je ne peux rien faire sans justificatif valable.." (Utilities|Array|MakeArray "Ok..")))
                      (switch Utilities|FlowControl|Switch|SwitchonEnum_DialogState _state_4
                        (:NewEnumerator0
                          (CallFunction|RemoveDialogueProgress 2)
                          (CallFunction|CloseConversation))))))))
            (:1
              (bind _state_5 (CallFunction|AddDialogue "Enzo Danthon" "ça va super merci. T'as loupé le coche, le prochain est prévu l'année prochaine vers mars !" (Utilities|Array|MakeArray "Ah dommage..")))
              (switch Utilities|FlowControl|Switch|SwitchonEnum_DialogState _state_5
                (:NewEnumerator0
                  (CallFunction|ClearDialogueProgress)
                  (CallFunction|CloseConversation))))))))
    (:1
      (bind _state_6 (CallFunction|AddDialogue "Enzo Danthon" (Utilities|Select :Index (Math|Random|RandomIntegerinRange 0 1) :Option%200 "C'est justifié je t'ai dit.. allez ouste" :Option%201 "Si tu reste planté là, je t'inscris au campus-cup") (Utilities|Array|MakeArray "Ok..")))
      (switch Utilities|FlowControl|Switch|SwitchonEnum_DialogState _state_6
        (:NewEnumerator0
          (CallFunction|ClearDialogueProgress)
          (CallFunction|CloseConversation))))))