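; NPC_Base is a base Blueprint for interactible NPCs that display a name label and an interact icon.
; The construction script writes CharacterName into the name text.
; SetInteractibleState shows or hides both the label and the icon.
; When a conversation closes, the NPC forwards ConversationClosedMessage to its InteractInstigator.
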(event EventSetInteractibleState
  (params (bCanShowInteract? :type Boolean))
  (if bCanShowInteract?
    (Rendering|SetVisibility (Variables|Default|GetTxt_CharacterName) true false)
    (Rendering|SetVisibility (Variables|Default|GetEIcon) true false)
    (else
      (Rendering|SetVisibility (Variables|Default|GetTxt_CharacterName) false false)
      (Rendering|SetVisibility (Variables|Default|GetEIcon) false false))))

(event EventConversationClosed
  (Class|BPIInteractable|ConversationClosed(Message) (Variables|Default|GetInteractInstigator)))

(fn ConstructionScript
  (Rendering|Components|TextRender|SetText (Variables|Default|GetTxt_CharacterName) (Variables|Default|GetCharacterName)))