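; Dialogue Blueprint for the NPC Eric Husson: a French, school-themed conversation about requesting remote classes or asking about an apprenticeship search.
; Overrides Dialogue, calls the parent, then switches on DialogueTreeIndex to chain AddDialogue nodes branching on the chosen option.
; An accepted remote request advances the tree to index 1, which plays one of two random dismissive or teasing lines.
; Other endings clear or roll back dialogue progress before closing the conversation.
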(fn Dialogue
  (|CallParentFunction)
  (switch int (Variables|Default|GetDialogueTreeIndex)
    (:0
      (bind (_state _optionindex) (CallFunction|AddDialogue "Eric Husson" "Bonjour, comment puis-je t'aider ?" (Utilities|Array|MakeArray "Boujour, je voudrais être en distanciel pour tous mes prochains cours svp !" "Bonjour, y a-t-il du nouveau concernant ma recherche d'alternance ? ")))
      (switch Utilities|FlowControl|Switch|SwitchonEnum_DialogState _state
        (:NewEnumerator0
          (switch int _optionindex
            (:0
              (bind (_state_2 _optionindex_2) (CallFunction|AddDialogue "Eric Husson" "humm.. C'est une très grosse demande que tu me fais là ! Quel est le motif ?" (Utilities|Array|MakeArray "Je vais être oppéré de mes deux jambes et je serais en fauteil pendant 6 mois... :(" "Franchement j'ai la flemme de venir en classe.. je préfère être sur teams :)")))
              (switch Utilities|FlowControl|Switch|SwitchonEnum_DialogState _state_2
                (:NewEnumerator0
                  (switch int _optionindex_2
                    (:0
                      (bind _state_3 (CallFunction|AddDialogue "Eric Husson" "Ah ! Force à toi dans cette épreuve, ta demande est légitime et sera acceptée !" (Utilities|Array|MakeArray "Merci !")))
                      (switch Utilities|FlowControl|Switch|SwitchonEnum_DialogState _state_3
                        (:NewEnumerator0
                          (CallFunction|SetDialogTreeIndex 1)
                          (CallFunction|CloseConversation))))
                    (:1
                      (bind _state_4 (CallFunction|AddDialogue "Eric Husson" "Mais t'as craqué jeune homme ? On ne paye pas des locaux pour rien ! Tu vas gentiment continue à venir à l'école !! " (Utilities|Array|MakeArray "Ok..")))
                      (switch Utilities|FlowControl|Switch|SwitchonEnum_DialogState _state_4
                        (:NewEnumerator0
                          (CallFunction|RemoveDialogueProgress 2)
                          (CallFunction|CloseConversation))))))))
            (:1
              (bind _state_5 (CallFunction|AddDialogue "Eric Husson" "Ah non, pas du tout, c'est encore au point mort... Mais ne t'inquiète pas, fait du 7speaking en attendant :)" (Utilities|Array|MakeArray "D'accord..")))
              (switch Utilities|FlowControl|Switch|SwitchonEnum_DialogState _state_5
                (:NewEnumerator0
                  (CallFunction|ClearDialogueProgress)
                  (CallFunction|CloseConversation))))))))
    (:1
      (bind _state_6 (CallFunction|AddDialogue "Eric Husson" (Utilities|Select :Index (Math|Random|RandomIntegerinRange 0 1) :Option%200 "T'as eu ce que tu voulais non ? Alors circule !" :Option%201 "Profite de ta convalescence pour faire du 7speaking ;)") (Utilities|Array|MakeArray "Ok..")))
      (switch Utilities|FlowControl|Switch|SwitchonEnum_DialogState _state_6
        (:NewEnumerator0
          (CallFunction|ClearDialogueProgress)
          (CallFunction|CloseConversation))))))